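; HUD Blueprint that draws the Botte_01 texture at the player's mouse position, acting as a custom cursor image.
; Each DrawHUD call reads the mouse position from player controller 0 and shifts it by half the difference between the HUD size and the viewport size.
; The centering offset is a literal zero, so the texture's top-left corner sits at that computed point.
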(event `self.ReceiveDrawHUD`
  (params (SizeX :type Integer) (SizeY :type Integer))
  (bind _returnvalue (`GameplayStatics.GetPlayerController` 0))
  (bind (_sizex _sizey) (`PlayerController.GetViewportSize` _returnvalue))
  (bind _returnvalue_2 (/ 0.0 2.0))
  (bind (_locationx _locationy) (`PlayerController.GetMousePosition` _returnvalue))
  (`self.DrawTextureSimple` "/Game/Assets/Thumbnails/Botte_01.Botte_01" (- (+ _locationx (/ (`KismetMathLibrary.Conv_IntToDouble` (- SizeX _sizex)) 2.0)) _returnvalue_2) (- (+ _locationy (/ (`KismetMathLibrary.Conv_IntToDouble` (- SizeY _sizey)) 2.0)) _returnvalue_2)))

(fn `UserConstructionScript`)