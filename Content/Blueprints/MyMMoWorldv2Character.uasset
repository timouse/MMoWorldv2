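; Player character Blueprint for an MMO project that sets up starting money and spell UI on BeginPlay.
; It copies the starting money to the player controller, adds a placeholder spell until a spellbook exists, then builds the spell bar widget from the spell array.
; A SetCastBarre event, called from C++, creates and displays the cast bar widget.
; The portrait creation call is disconnected and never runs.
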(event `self.ReceiveBeginPlay`
  (bind _asmy_mmo_worldv_2controller (cast `/Game/Blueprints/MyMMoWorldv2Controller` (`GameplayStatics.GetPlayerController` 0)))
  ;[1 0.2282 0.9774] A la création du personnage on ajoute un spell(a modifier plutard) on affiche le portrait joueur  on crée et affiche la barre des sort
  (set `MMoWorldv2Controller.Money` (`self.argent de depart`) _asmy_mmo_worldv_2controller)
  (bind _returnvalue (`self.AddSpell` "1")) ; a la création on ajoute un spell dans la barre , alternative en attendant de codé le grimoire des sort
  (if _returnvalue
    (bind _asmy_mmo_worldv_2controller_2 (cast `/Game/Blueprints/MyMMoWorldv2Controller` (`GameplayStatics.GetPlayerController` 0)))
    (bind _returnvalue_2 (`|CreateWidget` "/Game/Ui/WB_BarreSpell.WB_BarreSpell_C" (`GameplayStatics.GetPlayerController` 0)))
    (if (`KismetSystemLibrary.IsValid` _returnvalue_2)
      (set `/Game/Ui/WB_BarreSpell.ArraySpell` (`self.m_SpellBarre`) _returnvalue_2)
      (`UserWidget.AddToViewport` _returnvalue_2 0))))

(event `self.SetCastBarre`
  (params (Time :type "Float (single-precision)"))
  ;[1 0.3265 0.9807] Cast Barre appelé en c++ on crée l'interface de la barre de cast
  (bind _returnvalue (`|CreateWidget` "/Game/Ui/WB_CastBarre.WB_CastBarre_C" (`GameplayStatics.GetPlayerController` 0)))
  (`UserWidget.AddToViewport` _returnvalue 0))

(fn `UserConstructionScript`)