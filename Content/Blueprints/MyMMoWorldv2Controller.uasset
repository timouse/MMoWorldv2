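; Player controller for an MMO that owns the HUD widget and manages its target, loot, vendor, character sheet and inventory windows.
; BeginPlay creates the HUD and portrait, while Tick creates or updates the target window whenever a target is set.
; Left-clicking elsewhere clears the target and closes loot and vendor windows, guarded by overlay flags.
; Input actions toggle the character sheet and bag, and refresh events rebuild windows by destroying and recreating them.
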(event `self.ReceiveBeginPlay`
  (bind _returnvalue (`GameplayStatics.GetPlayerController` 0))
  (`/Engine/EditorBlueprintResources/StandardMacros.IsValid` _returnvalue
    (:`Is Valid`
      (bind _returnvalue_2 (`|CreateWidget` "/Game/Ui/WB_HudBase.WB_HudBase_C" _returnvalue))
      (bind _output_get (set `self.hud` _returnvalue_2))
      (`UserWidget.AddToViewport` _output_get 0)
      (`UserWidget.AddToViewport` _returnvalue_2 0)
      (`/Game/Ui/WB_HudBase.CreationPortrait` _output_get))))

(event `self.ReceiveTick`
  (params (DeltaSeconds :type "Float (single-precision)"))
  ;[0.9427 0.3103 1] Crée la fenêtre de la cible
  (if (`self.Cible`)
    (if (`self.WidgetDéjaCrée`)
      (set `/Game/Ui/WB_Cible.controller` self (`/Game/Ui/WB_HudBase.Cible` (`self.hud`)))
      (else
        (`/Game/Ui/WB_HudBase.CreeCible` (`self.hud`) self)
        (set `self.WidgetDéjaCrée` true)))))

(event `Key|LeftMouseButton`
  (params (Key :type "Key Structure"))
  ;[1 0.03839 0.8441] Detruit les fenetres de cible et de loot avec un click "autre part"
  (:`Pressed`
    (if (`self.WidgetDéjaCrée`)
      (if (or (`self.Overlay`) (`self.overlayvendeur`))
        _
        (elif (== (`self.Mob_copie`) (`self.mob copie_tempon`))
          _
          (elif (`KismetSystemLibrary.IsValid` (`self.mob copie_tempon`))
            (set `self.Mob_copie` (`self.mob copie_tempon`))
            (else
              (set `self.Mob_copie` null)
              (`/Game/Ui/WB_HudBase.DetruireCible` (`self.hud`))
              (set `self.Cible` false)
              (set `self.WidgetDéjaCrée` false)
              (if (`self.WB_loot`)
                (`Widget.RemoveFromParent` (`self.loot_widget`))
                (set `self.WB_loot` false))
              ;[1 0.04774 0.9966] detruit la fenetre si il y a un click "autre part" et que  le mob selectionné est un vendeur
              (if (`self.WB_Vendor`)
                (if (not (`self.overlayvendeur`))
                  (`/Game/Ui/WB_HudBase.DetruireFenetreVendeur` (`self.hud`))
                  (set `self.WB_Vendor` false))))))))))

(event `InputAction|OpenFichePersonnage`
  (params (Key :type "Key Structure"))
  (:`Pressed`
    (if (`self.FenetrePersonnageOuverte`)
      (`/Game/Ui/WB_HudBase.DestructionFenetrePersonnage` (`self.hud`))
      (set `self.FenetrePersonnageOuverte` false)
      (else
        (bind _asmy_mmo_worldv_2character (cast `/Game/Blueprints/MyMMoWorldv2Character` (`GameplayStatics.GetPlayerCharacter` 0)))
        (`/Game/Ui/WB_HudBase.CreationFenetrePersonnage` (`self.hud`) _asmy_mmo_worldv_2character)
        (set `self.FenetrePersonnageOuverte` true)))))

(event `InputAction|OpenInventory`
  (params (Key :type "Key Structure"))
  ;[0.969 0.3804 1] Affiche l'inventaire sur l'appuie de la touche associer "b" par default
  (:`Pressed`
    (if (`self.Sac_ouvert_fermer`)
      (set `self.Sac_ouvert_fermer` false)
      (`/Game/Ui/WB_HudBase.DetruireSac` (`self.hud`))
      (else
        (set `self.Sac_ouvert_fermer` true)
        (`/Game/Ui/WB_HudBase.CreationSac` (`self.hud`) (`self.Money`))))))

(event `Refresh sac`
  (bind _hud (`self.hud`))
  ;[1 1 1] Refresh le sac lors d'un nouvel ajout
  (`/Game/Ui/WB_HudBase.DetruireSac` _hud)
  (`/Game/Ui/WB_HudBase.CreationSac` _hud (`self.Money`))
  (set `self.sac refreshed` true)
  (set `self.Sac_ouvert_fermer` true))

(event `refreshFichePersonnage`
  (bind _asmy_mmo_worldv_2character (cast `/Game/Blueprints/MyMMoWorldv2Character` (`GameplayStatics.GetPlayerCharacter` 0)))
  (`/Game/Ui/WB_HudBase.DestructionFenetrePersonnage` (`self.hud`))
  (`/Game/Ui/WB_HudBase.CreationFenetrePersonnage` (`self.hud`) _asmy_mmo_worldv_2character)
  (set `self.FenetrePersonnageOuverte` true))

(event `RefreshVendeur`
  (bind _hud (`self.hud`))
  (bind _asmy_mmo_worldv_2mob_vendor (cast `/Game/Blueprints/MyMMoWorldv2Mob_Vendor` (`self.Mob_copie`)))
  (`/Game/Ui/WB_HudBase.DetruireFenetreVendeur` _hud)
  (`/Game/Ui/WB_HudBase.CreationFenetreVendeur` _hud _asmy_mmo_worldv_2mob_vendor))

(fn `UserConstructionScript`)