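; Vendor NPC mob that handles mouse hover and click on its cube, reporting to the player controller.
; Hover sets the controller's overlay flag and temporary mob reference.
; A click opens a loot widget if the mob is dead and makes it the target if none is set.
; It also has the HUD open the vendor window, unless already flagged open, when the mob is inside the character's collision sphere.
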(event `self.Cube.OnClicked`
  (params (TouchedComponent :type "PrimitiveComponent Object Reference") (ButtonPressed :type "Key Structure"))
  ;[1 1 1] crée la cible et sa fenettre de loot si il est mort
  (bind _asmy_mmo_worldv_2controller (cast `/Game/Blueprints/MyMMoWorldv2Controller` (`GameplayStatics.GetPlayerController` 0)))
  (bind _returnvalue (`self.Get_Life`))
  (if (not (> _returnvalue 0))
    (bind _returnvalue_2 (`|CreateWidget` "/Game/Ui/WB_Loot.WB_Loot_C" (`GameplayStatics.GetPlayerController` 0)))
    (bind _returnvalue_3 (`self.Get_loot_item`))
    (`/Game/Ui/WB_Loot.Set loot` _returnvalue_2 _returnvalue_3)
    (set `/Game/Blueprints/MyMMoWorldv2Controller.loot_widget` _returnvalue_2 _asmy_mmo_worldv_2controller)
    (`UserWidget.AddToViewport` _returnvalue_2 0)
    (set `/Game/Blueprints/MyMMoWorldv2Controller.WB_loot` true _asmy_mmo_worldv_2controller))
  (if (not (`MMoWorldv2Controller.Cible` _asmy_mmo_worldv_2controller))
    (set `MMoWorldv2Controller.Mob_copie` self _asmy_mmo_worldv_2controller)
    (set `MMoWorldv2Controller.Cible` true _asmy_mmo_worldv_2controller))
  ;[1 1 1] gestion de l'affichge de l'interface du vendeur
  (if (not (`/Game/Blueprints/MyMMoWorldv2Controller.WB_Vendor` _asmy_mmo_worldv_2controller))
    ;;[1 1 1] ici on regarde si la cible est dans la sphere collision , en gros si le pnj est pas loin, si c'est le cas on affiche la fenetre
    (bind _asmy_mmo_worldv_2character (cast `/Game/Blueprints/MyMMoWorldv2Character` (`GameplayStatics.GetPlayerCharacter` 0)))
    (bind _returnvalue_4 (`MMoWorldv2Character.CheckSphereCollision` _asmy_mmo_worldv_2character))
    (for _array_element _returnvalue_4
      (if (== _array_element self)
        (bind _asmy_mmo_worldv_2controller_2 (cast `/Game/Blueprints/MyMMoWorldv2Controller` (`GameplayStatics.GetPlayerController` 0)))
        (`/Game/Ui/WB_HudBase.CreationFenetreVendeur` (`/Game/Blueprints/MyMMoWorldv2Controller.hud` _asmy_mmo_worldv_2controller_2) self)
        (set `/Game/Blueprints/MyMMoWorldv2Controller.WB_Vendor` true _asmy_mmo_worldv_2controller_2)))))

(event `self.Cube.OnBeginCursorOver`
  (params (TouchedComponent :type "PrimitiveComponent Object Reference"))
  ;[1 1 1] met a jour la variable dans controller pour savoir si la cible est en overlay ou pas
  (bind _asmy_mmo_worldv_2controller (cast `/Game/Blueprints/MyMMoWorldv2Controller` (`GameplayStatics.GetPlayerController` 0)))
  (set `/Game/Blueprints/MyMMoWorldv2Controller.Overlay` true _asmy_mmo_worldv_2controller)
  (set `/Game/Blueprints/MyMMoWorldv2Controller.mob copie_tempon` self _asmy_mmo_worldv_2controller))

(event `self.Cube.OnEndCursorOver`
  (params (TouchedComponent :type "PrimitiveComponent Object Reference"))
  ;[1 1 1] met a jour la variable dans controller pour savoir si la cible est en overlay ou pas
  (bind _asmy_mmo_worldv_2controller (cast `/Game/Blueprints/MyMMoWorldv2Controller` (`GameplayStatics.GetPlayerController` 0)))
  (set `/Game/Blueprints/MyMMoWorldv2Controller.Overlay` false _asmy_mmo_worldv_2controller)
  (set `/Game/Blueprints/MyMMoWorldv2Controller.mob copie_tempon` null _asmy_mmo_worldv_2controller))

(fn `UserConstructionScript`)