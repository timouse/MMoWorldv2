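; BP_Mob is a clickable MMO mob actor that serves as the player's target and loot source.
; Clicking its mesh registers it as the controller's target if none is set, and opens a WB_Loot widget filled from GetLootItem when its life is depleted.
; Mesh hover events update the controller's mouse-over flag and temporary mob reference.
; A TextRender shows the mob's name, rotated every Tick to face the camera.
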(event `self.StaticMesh.OnClicked`
  (params (TouchedComponent :type "PrimitiveComponent Object Reference") (ButtonPressed :type "Key Structure"))
  (bind _mmoworldv2controller (`self.MMoworldv2controller`))
  (bind _mmoworldv2controller_2 (`self.MMoworldv2controller`))
  ;[1 0.1739 0.8357] fonction Click, au click sur le mob on cast vers controller et on lui affecte la cible si la cible est morte on crée l'ui de loot et on met a jour la table des loot ( fonction a revoir le widget n'est pas a crée ici mais dans le controller )
  (bind _asmy_mmo_worldv_2controller (cast `/Game/Blueprints/MyMMoWorldv2Controller` (`GameplayStatics.GetPlayerController` 0)))
  (set `self.MMoworldv2controller` _asmy_mmo_worldv_2controller)
  (bind _returnvalue (`self.Get_Life`))
  (if (not (> _returnvalue 0))
    (bind _returnvalue_2 (`|CreateWidget` "/Game/Ui/WB_Loot.WB_Loot_C" (`GameplayStatics.GetPlayerController` 0)))
    (bind _returnvalue_3 (`self.Get_loot_item`))
    (`/Game/Ui/WB_Loot.Set loot` _returnvalue_2 _returnvalue_3)
    (set `/Game/Blueprints/MyMMoWorldv2Controller.loot_widget` _returnvalue_2 _mmoworldv2controller_2)
    (`UserWidget.AddToViewport` _returnvalue_2 0)
    (set `/Game/Blueprints/MyMMoWorldv2Controller.WB_loot` true _mmoworldv2controller_2))
  (if (`MMoWorldv2Controller.Cible` (`self.MMoworldv2controller`))
    (if (== (`MMoWorldv2Controller.Mob_copie` (`self.MMoworldv2controller`)) self)
      _)
    (else
      (set `MMoWorldv2Controller.Mob_copie` self _mmoworldv2controller)
      (set `MMoWorldv2Controller.Cible` true _mmoworldv2controller))))

(event `self.ReceiveBeginPlay`
  (bind _returnvalue (`self.Get_Name`))
  (`TextRenderComponent.K2_SetText` (`self.TextRender`) (`KismetTextLibrary.Conv_StringToText` _returnvalue)))

(event `self.ReceiveTick`
  (params (DeltaSeconds :type "Float (single-precision)"))
  (bind _returnvalue (`GameplayStatics.GetPlayerCameraManager` 0))
  (bind (_returnvalue_roll _returnvalue_pitch _returnvalue_yaw) (`KismetMathLibrary.BreakRotator` (`KismetMathLibrary.Conv_VectorToRotator` (`self.GetActorForwardVector` _returnvalue))))
  (`/Engine/EditorBlueprintResources/StandardMacros.IsValid` _returnvalue
    (:`Is Valid`
      (`SceneComponent.K2_SetWorldRotation` (`self.TextRender`) (`KismetMathLibrary.MakeRotator` _returnvalue_roll _returnvalue_pitch (+ _returnvalue_yaw 180.0)) false false))))

(event `self.CapsuleComponent.OnBeginCursorOver`
  (params (TouchedComponent :type "PrimitiveComponent Object Reference"))
  ;[1 0.28 0.9833] Gère l'overlay du mob variable mouseOverlayMob 1/0
)

(event `self.StaticMesh.OnBeginCursorOver`
  (params (TouchedComponent :type "PrimitiveComponent Object Reference"))
  ;[1 0.28 0.9833] Gère l'overlay du mob variable mouseOverlayMob 1/0
  (bind _asmy_mmo_worldv_2controller (cast `/Game/Blueprints/MyMMoWorldv2Controller` (`GameplayStatics.GetPlayerController` 0)))
  (set `MMoWorldv2Controller.m_MouseOverlay_mob` true _asmy_mmo_worldv_2controller)
  (set `self.overlay` true)
  (set `/Game/Blueprints/MyMMoWorldv2Controller.mob copie_tempon` self _asmy_mmo_worldv_2controller))

(event `self.StaticMesh.OnEndCursorOver`
  (params (TouchedComponent :type "PrimitiveComponent Object Reference"))
  ;[1 0.28 0.9833] Gère l'overlay du mob variable mouseOverlayMob 1/0
  (bind _asmy_mmo_worldv_2controller (cast `/Game/Blueprints/MyMMoWorldv2Controller` (`GameplayStatics.GetPlayerController` 0)))
  (set `MMoWorldv2Controller.m_MouseOverlay_mob` false _asmy_mmo_worldv_2controller)
  (set `self.overlay` false)
  (set `/Game/Blueprints/MyMMoWorldv2Controller.mob copie_tempon` null _asmy_mmo_worldv_2controller))

(event `self.CapsuleComponent.OnEndCursorOver`
  (params (TouchedComponent :type "PrimitiveComponent Object Reference"))
  ;[1 0.28 0.9833] Gère l'overlay du mob variable mouseOverlayMob 1/0
)

(fn `UserConstructionScript`)